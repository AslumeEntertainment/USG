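; BP_ConsumableSpawner is a spawner actor that keeps one random consumable present at its socket location.
; On BeginPlay it spawns immediately and starts a looping timer at the SpawnTime interval.
; Each tick of the timer, only on the authority, it spawns a random class from ConsumableActorClasses at SpawnSocket if the last spawned actor is no longer valid.
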(event Custom|SpawnConsumable
  (if (Ability|HasAuthority)
    (Utilities|IsValid (Variables|Default|GetSpawnedActor)
      (:Is%20Not%20Valid
        (bind _returnvalue (Game|SpawnActorfromClass (.OutItem (Utilities|Array|Random (Variables|Default|GetConsumableActorClasses))) (Math|Conversions|ToTransform(Vector) (Transformation|GetWorldLocation (Variables|Default|GetSpawnSocket))) "Undefined" "MultiplyWithRoot" 0 0))
        (Variables|Default|SetSpawnedActor _returnvalue)))))

(event EventBeginPlay
  (CallFunction|SpawnConsumable)
  (Utilities|Time|SetTimerbyEvent (delegate Custom|SpawnConsumable) (Variables|Default|GetSpawnTime) true))

(fn ConstructionScript)